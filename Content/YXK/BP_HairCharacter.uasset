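; BP_HairCharacter is a hair character Blueprint that generates five continuously looping, phase-offset animation values, Location1X through Location5X.
; On BeginPlay, a Sequence starts five timelines at quarter-second stagger intervals, each writing its track output to its matching variable.
; Each timeline loops by calling a DoReplay custom event on Finished, which plays it from the start.
; Nothing in these graphs consumes the values.
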(event Custom|DoReplay5
  (bind _newtrack_0 (Timeline|Location5 PlayFromStart)
    (:Update
      (Variables|Default|SetLocation5X _newtrack_0))
    (:Finished
      (CallFunction|DoReplay5))))

(event Custom|DoReplay1
  (bind _newtrack_0 (Timeline|Location1 PlayFromStart)
    (:Update
      (Variables|Default|SetLocation1X _newtrack_0))
    (:Finished
      (CallFunction|DoReplay1))))

(event Custom|DoReplay2
  (bind _newtrack_0 (Timeline|Location2 PlayFromStart)
    (:Update
      (Variables|Default|SetLocation2X _newtrack_0))
    (:Finished
      (CallFunction|DoReplay2))))

(event Custom|DoReplay3
  (bind _newtrack_0 (Timeline|Location3 PlayFromStart)
    (:Update
      (Variables|Default|SetLocation3X _newtrack_0))
    (:Finished
      (CallFunction|DoReplay3))))

(event Custom|DoReplay4
  (bind _newtrack_0 (Timeline|Location4 PlayFromStart)
    (:Update
      (Variables|Default|SetLocation4X _newtrack_0))
    (:Finished
      (CallFunction|DoReplay4))))

(event EventBeginPlay
  (Utilities|FlowControl|Sequence
    (:then_0
      (bind _newtrack_0 (Timeline|Location1 Play)
        (:Update
          (Variables|Default|SetLocation1X _newtrack_0))
        (:Finished
          (CallFunction|DoReplay1))))
    (:then_1
      (Utilities|FlowControl|Delay 0.25)
      (bind _newtrack_0_2 (Timeline|Location2 Play)
        (:Update
          (Variables|Default|SetLocation2X _newtrack_0_2))
        (:Finished
          (CallFunction|DoReplay2))))
    (:then_2
      (Utilities|FlowControl|Delay 0.5)
      (bind _newtrack_0_3 (Timeline|Location3 Play)
        (:Update
          (Variables|Default|SetLocation3X _newtrack_0_3))
        (:Finished
          (CallFunction|DoReplay3))))
    (:then_3
      (Utilities|FlowControl|Delay 0.75)
      (bind _newtrack_0_4 (Timeline|Location4 Play)
        (:Update
          (Variables|Default|SetLocation4X _newtrack_0_4))
        (:Finished
          (CallFunction|DoReplay4))))
    (:then_4
      (Utilities|FlowControl|Delay 1.0)
      (bind _newtrack_0_5 (Timeline|Location5 Play)
        (:Update
          (Variables|Default|SetLocation5X _newtrack_0_5))
        (:Finished
          (CallFunction|DoReplay5))))))

(event Collision|EventActorBeginOverlap
  (params (OtherActor :type Actor%20Object%20Reference)))

(event EventTick
  (params (DeltaSeconds :type Float%20%28single-precision%29)))

(fn ConstructionScript)